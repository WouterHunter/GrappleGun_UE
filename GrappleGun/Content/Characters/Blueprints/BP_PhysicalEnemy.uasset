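; BP_PhysicalEnemy is an enemy that drives itself along its forward vector with simple hand-written momentum.
; Each Tick adds forward acceleration, scaled by Movespeed and DeltaSeconds, to Velocity, then scales the result's length by LinearDamping.
; Velocity is applied directly as a per-frame world offset on the root without sweep, so movement ignores blocking collision and damping depends on frame rate.
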(event `self.ReceiveTick`
  (params (DeltaSeconds :type "Float (single-precision)"))
  (bind _output_get (set `self.Acceleration` (* (* DeltaSeconds (`self.Movespeed`)) (`self.GetActorForwardVector`))))
  (bind _returnvalue (+ _output_get (`self.Velocity`)))
  (bind _output_get_2 (set `self.Velocity` (* (`KismetMathLibrary.Normal` _returnvalue) (* (`KismetMathLibrary.VSize` _returnvalue) (`self.LinearDamping`)))))
  (`SceneComponent.K2_AddWorldOffset` (`self.DefaultSceneRoot`) _output_get_2 false false))

(fn `UserConstructionScript`)