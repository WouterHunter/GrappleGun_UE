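; Actor component that gives its owner's skeletal mesh physical-animation hit reactions and can trigger full-body physics simulation.
; BeginPlay adds a PhysicalAnimationComponent and simulates below the pelvis using the "Strong" profile.
; HitReaction switches profile, adds reaction time and applies an impulse along the trace, redirecting pelvis hits to spine_02.
; Tick fades physics blend weight with remaining time, then stops simulation and ticking, though HitReaction also disables ticking rather than enabling it.
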(event `self.ReceiveBeginPlay`
  (bind _returnvalue (`self.GetOwner`))
  (bind _returnvalue_2 (`Actor.GetComponentByClass` _returnvalue "/Script/Engine.SkeletalMeshComponent"))
  (bind _returnvalue_3 (`|AddComponentByClass` _returnvalue "/Script/Engine.PhysicalAnimationComponent"))
  (bind _output_get (set `self.PhysAnimComp` _returnvalue_3))
  (`PhysicalAnimationComponent.SetSkeletalMeshComponent` _output_get _returnvalue_2)
  (bind _output_get_2 (set `self.SkelMeshComp` _returnvalue_2))
  (`SkeletalMeshComponent.SetAllBodiesBelowSimulatePhysics` _output_get_2 (`self.PelvisName`) true false)
  (`PhysicalAnimationComponent.ApplyPhysicalAnimationProfileBelow` (`self.PhysAnimComp`) (`self.PelvisName`) "Strong" false false))

(event `self.ReceiveTick`
  (params (DeltaSeconds :type "Float (single-precision)"))
  (bind _output_get (set `self.HitReactionTimeRemaining` (- (`KismetMathLibrary.FInterpTo` (`self.HitReactionTimeRemaining`) 0.0 0.0 1.0) (* DeltaSeconds 0.1))))
  (if (<= _output_get 0.0)
    (`SkeletalMeshComponent.SetAllBodiesBelowSimulatePhysics` (`self.SkelMeshComp`) (`self.PelvisName`) false true)
    (`self.SetComponentTickEnabled` false)
    (else
      (`SkeletalMeshComponent.SetAllBodiesBelowPhysicsBlendWeight` (`self.SkelMeshComp`) (`self.PelvisName`) (`KismetMathLibrary.FMin` (`self.HitReactionTimeRemaining`) 1.0) false true))))

(event `TriggerPhysicalAnimation`
  (bind _skelmeshcomp (`self.SkelMeshComp`))
  (`PrimitiveComponent.SetCollisionEnabled` _skelmeshcomp "QueryAndPhysics")
  (`SkeletalMeshComponent.SetAllBodiesSimulatePhysics` _skelmeshcomp true))

(event `HitReaction`
  (params (`Hit Result` :type "HitResult Structure"))
  (bind (_bblockinghit _binitialoverlap _time _distance _location _impactpoint _normal _impactnormal _physmat _hitactor _hitcomponent _hitbonename _bonename _hititem _elementindex _faceindex _tracestart _traceend) (`GameplayStatics.BreakHitResult` `Hit Result`))
  (`self.SetComponentTickEnabled` false)
  (set `self.HitReactionTimeRemaining` (+ (`self.HitReactionTimeRemaining`) 2.0))
  (`PhysicalAnimationComponent.ApplyPhysicalAnimationProfileBelow` (`self.PhysAnimComp`) (`self.PelvisName`) "HitReactionProfile" false false)
  (`SkeletalMeshComponent.SetAllBodiesBelowSimulatePhysics` (`self.SkelMeshComp`) (`self.PelvisName`) true false)
  (`PrimitiveComponent.AddImpulse` (`self.SkelMeshComp`) (* (`self.ImpulseStrength`) (`KismetMathLibrary.Normal` (- _traceend _tracestart))) (select `bool` (== _hitbonename (`self.PelvisName`)) :`false` _hitbonename :`true` "spine_02") false))