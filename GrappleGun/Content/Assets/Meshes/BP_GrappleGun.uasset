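; Grapple gun actor that keeps four pivot components aimed at two referenced target actors.
; Pivot and Pivot1 face Target1, while Pivot2 and Pivot3 face Target2, each using a look-at rotation plus a fixed relative offset to correct orientation.
; The same logic runs in the Construction Script and every Tick, so the aim updates both on construction and during play.
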(event `self.ReceiveTick`
  (params (DeltaSeconds :type "Float (single-precision)"))
  (`SceneComponent.K2_SetWorldRotation` (`self.Pivot`) (`KismetMathLibrary.FindLookAtRotation` (`SceneComponent.K2_GetComponentLocation` (`self.Pivot`)) (`self.K2_GetActorLocation` (`self.Target_1`))) false false)
  (`SceneComponent.K2_AddRelativeRotation` (`self.Pivot`) (struct :`Yaw` 180.0) false false)
  (`SceneComponent.K2_SetWorldRotation` (`self.Pivot 1`) (`KismetMathLibrary.FindLookAtRotation` (`SceneComponent.K2_GetComponentLocation` (`self.Pivot 1`)) (`self.K2_GetActorLocation` (`self.Target_1`))) false false)
  (`SceneComponent.K2_AddRelativeRotation` (`self.Pivot 1`) (struct :`Yaw` 270.0) false false)
  (`SceneComponent.K2_SetWorldRotation` (`self.Pivot2`) (`KismetMathLibrary.FindLookAtRotation` (`SceneComponent.K2_GetComponentLocation` (`self.Pivot2`)) (`self.K2_GetActorLocation` (`self.Target_2`))) false false)
  (`SceneComponent.K2_AddRelativeRotation` (`self.Pivot2`) (struct :`Yaw` 270.0) false false)
  (`SceneComponent.K2_SetWorldRotation` (`self.Pivot3`) (`KismetMathLibrary.FindLookAtRotation` (`SceneComponent.K2_GetComponentLocation` (`self.Pivot3`)) (`self.K2_GetActorLocation` (`self.Target_2`))) false false)
  (`SceneComponent.K2_AddRelativeRotation` (`self.Pivot3`) (struct :`Yaw` 270.0) false false))

(fn `UserConstructionScript`
  (`SceneComponent.K2_SetWorldRotation` (`self.Pivot`) (`KismetMathLibrary.FindLookAtRotation` (`SceneComponent.K2_GetComponentLocation` (`self.Pivot`)) (`self.K2_GetActorLocation` (`self.Target_1`))) false false)
  (`SceneComponent.K2_AddRelativeRotation` (`self.Pivot`) (struct :`Yaw` 180.0) false false)
  (`SceneComponent.K2_SetWorldRotation` (`self.Pivot 1`) (`KismetMathLibrary.FindLookAtRotation` (`SceneComponent.K2_GetComponentLocation` (`self.Pivot 1`)) (`self.K2_GetActorLocation` (`self.Target_1`))) false false)
  (`SceneComponent.K2_AddRelativeRotation` (`self.Pivot 1`) (struct :`Yaw` 270.0) false false)
  (`SceneComponent.K2_SetWorldRotation` (`self.Pivot2`) (`KismetMathLibrary.FindLookAtRotation` (`SceneComponent.K2_GetComponentLocation` (`self.Pivot2`)) (`self.K2_GetActorLocation` (`self.Target_2`))) false false)
  (`SceneComponent.K2_AddRelativeRotation` (`self.Pivot2`) (struct :`Yaw` 270.0) false false)
  (`SceneComponent.K2_SetWorldRotation` (`self.Pivot3`) (`KismetMathLibrary.FindLookAtRotation` (`SceneComponent.K2_GetComponentLocation` (`self.Pivot3`)) (`self.K2_GetActorLocation` (`self.Target_2`))) false false)
  (`SceneComponent.K2_AddRelativeRotation` (`self.Pivot3`) (struct :`Yaw` 270.0) false false))